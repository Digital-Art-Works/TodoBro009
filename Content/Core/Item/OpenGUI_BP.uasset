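; OpenGUI_BP is a trigger actor that offers the player an interact button for opening a configurable menu.
; When MyPlayer overlaps its Box, it passes TooltipText and GUIToOpen to MyHUD's DisplayInteractButton as the button title and next menu.
; Leaving the Box hides the button and switches the HUD to the menu enum's NewEnumerator0 entry.
; The HUD is always taken from player controller 0.
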(event OnComponentBeginOverlap(Box)
  (params (OverlappedComponent :type Primitive%20Component%20Object%20Reference) (OtherActor :type Actor%20Object%20Reference) (OtherComp :type Primitive%20Component%20Object%20Reference) (OtherBodyIndex :type Integer) (bFromSweep :type Boolean) (SweepResult :type Hit%20Result%20Structure%20%28by%20ref%29))
  (Utilities|Casting|CastToMyPlayer OtherActor)
  (bind _asmy_hud (Utilities|Casting|CastToMyHUD (HUD|GetHUD (Game|GetPlayerController 0))))
  (Default|DisplayInteractButton _asmy_hud (Variables|Default|GetTooltip%20Text) (Variables|Default|GetGUI%20to%20open)))

(event OnComponentEndOverlap(Box)
  (params (OverlappedComponent :type Primitive%20Component%20Object%20Reference) (OtherActor :type Actor%20Object%20Reference) (OtherComp :type Primitive%20Component%20Object%20Reference) (OtherBodyIndex :type Integer))
  (Utilities|Casting|CastToMyPlayer OtherActor)
  (bind _asmy_hud (Utilities|Casting|CastToMyHUD (HUD|GetHUD (Game|GetPlayerController 0))))
  (Default|HideInteractButton _asmy_hud)
  (Default|ChangeMenu _asmy_hud "NewEnumerator0"))

(event EventBeginPlay)

(event Collision|EventActorBeginOverlap
  (params (OtherActor :type Actor%20Object%20Reference)))

(event EventTick
  (params (DeltaSeconds :type Float%20%28single-precision%29)))

(fn ConstructionScript)